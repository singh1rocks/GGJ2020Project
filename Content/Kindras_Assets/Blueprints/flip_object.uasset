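; Actor Blueprint that rocks an object back and forth around its roll axis.
; Tick adds RotationRate to the roll every frame, without delta-time scaling, so speed depends on frame rate.
; BeginPlay calls SwitchRotation, which uses a FlipFlop to alternate the rate's sign and sets a looping timer on itself to reverse direction at a fixed interval.
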(event Custom|SwitchRotation
  (Utilities|FlowControl|FlipFlop
    (:A
      (Variables|Default|SetRotationRate 1.0))
    (:B
      (Variables|Default|SetRotationRate -1.0)))
  (Utilities|Time|SetTimerbyEvent (delegate Custom|SwitchRotation) 2.0 true))

(event EventBeginPlay
  (CallFunction|SwitchRotation))

(event EventTick
  (params (DeltaSeconds :type Float%20%28single-precision%29))
  (bind _returnvalue (Transformation|GetActorRotation))
  (bind (_roll _pitch _yaw) (Math|Rotator|BreakRotator _returnvalue))
  (Transformation|SetActorRotation (Math|Rotator|MakeRotator (+ _roll (Variables|Default|GetRotationRate)) _pitch _yaw)))

(fn ConstructionScript)