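; NextLvl_BP is a next-level actor that ends a level when its objective is met and moves the game on.
; The Mice check event decrements a counter; at zero it prints a win message, waits briefly, then opens the Village level.
; The Cat check only prints the win message, while the Ogre, Lakers and Cave checks are empty stubs, with leftover unconnected Village load nodes.
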(event Custom|Check%20for%20next%20level%20Mice
  (Variables|Default|SetCount (- (Variables|Default|GetCount) 1))
  (if (<= (Variables|Default|GetCount) 0)
    (Development|PrintString "YOU WIN")
    (Utilities|FlowControl|Delay 3.0)
    (Game|OpenLevel(byName) "Village")))

(event Custom|Check%20for%20next%20level%20Ogre)

(event Custom|Check%20For%20next%20level%20Lakers)

(event Custom|Check%20for%20next%20level%20Cave)

(event Custom|Check%20for%20next%20level%20Cat
  (Development|PrintString "YOU WIN"))

(fn ConstructionScript)