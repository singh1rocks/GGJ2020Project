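; Spinning, hovering switch actor that, when activated, updates the player's cheese and changes its own appearance.
; A looping one-second FlipFlop toggles the bob direction, while Tick rotates and moves the mesh by fixed per-frame steps.
; SendActivation calls UpdateCheese on the FirstPersonCharacter cached at BeginPlay, then swaps in the Battery mesh with a cheese material.
; A separate event increments CheeseCount directly, outside the activation path.
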(event Custom|Send%20Cheese%20to%20Player
  (bind _player_ref (Variables|Default|GetPlayer%20Ref))
  (Variables|/Game/FirstPersonBP/Blueprints/FirstPersonCharacter.FirstPersonCharacter_C|SetCheeseCount _player_ref (+ (Variables|/Game/FirstPersonBP/Blueprints/FirstPersonCharacter.FirstPersonCharacter_C|GetCheeseCount _player_ref) 1)))

(event Custom|Hover
  (Utilities|FlowControl|FlipFlop :!label _label
    (:A
      (Variables|Default|SetUp? false))
    (:B
      (Variables|Default|SetUp? true)))
  (Utilities|FlowControl|Delay 1.0)
  (goto _label))

(event Custom|SwapCheese
  (bind _staticmesh (Variables|Default|GetStaticmesh))
  (Components|StaticMesh|SetStaticMesh _staticmesh "/Game/Logans_Assets/Villagers_and_Enemies/battery.battery")
  (Rendering|Material|SetMaterial _staticmesh 0 "/Game/Logans_Assets/Villagers_and_Enemies/Cheese_Mat.Cheese_Mat"))

(event EventBeginPlay
  (bind _asfirst_person_character (Utilities|Casting|CastToFirstPersonCharacter (Game|GetPlayerCharacter 0)))
  (Variables|Default|SetPlayer%20Ref _asfirst_person_character)
  (CallFunction|Hover))

(event EventTick
  (params (DeltaSeconds :type Float%20%28single-precision%29))
  (Transformation|AddRelativeRotation (Variables|Default|GetStaticmesh) "0.000000,1.000000, 0" false false)
  (if (Variables|Default|GetUp?)
    (Transformation|AddRelativeLocation (Variables|Default|GetStaticmesh) (Math|Vector|MakeVector 0.0 0.0 0.15) false false)
    (else
      (Transformation|AddRelativeLocation (Variables|Default|GetStaticmesh) (Math|Vector|MakeVector 0.0 0.0 -0.15) false false))))

(event EventSendActivation
  (params (Activate? :type Boolean))
  (Default|UpdateCheese (Variables|Default|GetPlayer%20Ref))
  (CallFunction|SwapCheese))

(fn ConstructionScript)